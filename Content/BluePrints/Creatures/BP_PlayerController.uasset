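; BP_PlayerController is the player controller that turns movement input into state and facing for the controlled BP_Knight.
; It caches the knight on BeginPlay, then runs UpdateInput every Tick.
; While Idle or Move, both sharing one logic path, it picks Move or Idle from the up/right axes and sets Direction from their signs.
; Horizontal input is evaluated last, so it overrides vertical facing on diagonals.
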(event EventBeginPlay
  (bind _asbp_knight (Utilities|Casting|CastToBP_Knight (Pawn|GetControlledPawn)))
  (Variables|Default|SetMyPlayer _asbp_knight))

(event EventTick
  (params (DeltaSeconds :type Float%20%28single-precision%29))
  (CallFunction|UpdateInput))

(fn ConstructionScript)

(fn UpdateInput
  (switch Utilities|FlowControl|Switch|SwitchonEState (Variables|/Game/BluePrints/Creatures/BP_Creature.BP_Creature_C|GetState (Variables|Default|GetMyPlayer))
    (:NewEnumerator0
      _)
    (:NewEnumerator1
      _))
  (Utilities|FlowControl|Sequence
    (:then_0
      (if (or (!= (Input|AxisValues|GetMoveUp) 0.0) (!= (Input|AxisValues|GetMoveRight) 0.0))
        (Variables|/Game/BluePrints/Creatures/BP_Creature.BP_Creature_C|SetState (Variables|Default|GetMyPlayer) "NewEnumerator1")
        (else
          (Variables|/Game/BluePrints/Creatures/BP_Creature.BP_Creature_C|SetState (Variables|Default|GetMyPlayer) "NewEnumerator0"))))
    (:then_1
      (Math|Float|CompareFloat (Input|AxisValues|GetMoveUp) 0.0
        (:>
          (Variables|/Game/BluePrints/Creatures/BP_Creature.BP_Creature_C|SetDirection (Variables|Default|GetMyPlayer) "NewEnumerator0"))
        (:<
          (Variables|/Game/BluePrints/Creatures/BP_Creature.BP_Creature_C|SetDirection (Variables|Default|GetMyPlayer) "NewEnumerator1"))))
    (:then_2
      (Math|Float|CompareFloat (Input|AxisValues|GetMoveRight) 0.0
        (:>
          (Variables|/Game/BluePrints/Creatures/BP_Creature.BP_Creature_C|SetDirection (Variables|Default|GetMyPlayer) "NewEnumerator3"))
        (:<
          (Variables|/Game/BluePrints/Creatures/BP_Creature.BP_Creature_C|SetDirection (Variables|Default|GetMyPlayer) "NewEnumerator2"))))))