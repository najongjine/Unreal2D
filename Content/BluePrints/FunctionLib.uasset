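; A Blueprint function library of shortcut lookups for the project's core objects.
; GetBPGameInstance and GetBPGameMode return the game instance and game mode cast to BP_GameInstance and BP_GameMode.
; GetBPTileMap searches the level for a BP_TileMap actor with GetActorOfClass but does not pass the result to its return.
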(fn GetBPGameInstance
  (bind _asbp_game_instance (Utilities|Casting|CastToBP_GameInstance (Game|GetGameInstance)))
  (return _asbp_game_instance))

(fn GetBPTileMap
  (Actor|GetActorOfClass 0 "/Game/BluePrints/BP_Tilemap.BP_TileMap_C")
  (return 0))

(fn GetBPGameMode
  (bind _asbp_game_mode (Utilities|Casting|CastToBP_GameMode (Game|GetGameMode)))
  (return _asbp_game_mode))